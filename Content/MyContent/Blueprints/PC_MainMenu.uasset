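; Player controller for the main menu that creates the menu's widgets for the local player.
; On BeginPlay it creates and stores the main menu, create server and server browser widgets, adding only the main menu to the viewport.
; A ToggleMouseCursor input branches on a constant true, so it always shows the cursor and never reaches the hide path.
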(event `self.ReceiveBeginPlay`
  (if (`self.IsLocalPlayerController`)
    (bind _returnvalue (`|CreateWidget` "/Game/MyContent/UI/WB_MainMenu.WB_MainMenu_C"))
    (bind _output_get (set `self.WB_MainMenu` _returnvalue))
    (`UserWidget.AddToViewport` _output_get 0)
    (bind _returnvalue_2 (`|CreateWidget` "/Game/MyContent/UI/WB_CreateServer.WB_CreateServer_C"))
    (set `self.WB_CreateServer` _returnvalue_2)
    (bind _returnvalue_3 (`|CreateWidget` "/Game/MyContent/UI/WB_ServerBrowser.WB_ServerBrowser_C"))
    (set `self.WB_ServerBrowser` _returnvalue_3)))

(event `InputAction|ToggleMouseCursor`
  (params (Key :type "Key Structure"))
  (:`Pressed`
    (if true
      (set `self.bShowMouseCursor` true)
      (set `self.IsCursorVisible` false)
      (else
        (set `self.bShowMouseCursor` false)
        (set `self.IsCursorVisible` true)))))

(fn `UserConstructionScript`)